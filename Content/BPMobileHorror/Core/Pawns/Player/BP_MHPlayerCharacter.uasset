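; Player character for a mobile horror game that detects and uses interactable actors through BPI_MHInteractInterface.
; Capsule overlaps toggle an in-sight flag and send ready-to-use messages to interface actors entering or leaving range.
; While flagged, Tick sphere-traces from the camera, with debug drawing, over the capsule's full height to pick the target actor.
; ActionUse sends that target the interact message and prints the result on screen.
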(event `self.ReceiveBeginPlay`
  (`parent.ReceiveBeginPlay`)
  (`self.UpdateInteractionRadius`))

(event `self.ReceiveTick`
  (params (DeltaSeconds :type "Float (single-precision)"))
  (`parent.ReceiveTick` DeltaSeconds)
  (`self.CheckInteractionActorInSight`))

(event `self.InteractCapsule.OnComponentBeginOverlap`
  (params (OverlappedComponent :type "PrimitiveComponent Object Reference") (OtherActor :type "Actor Object Reference") (OtherComp :type "PrimitiveComponent Object Reference") (OtherBodyIndex :type Integer) (bFromSweep :type Boolean) (SweepResult :type "HitResult Structure (by ref)"))
  (if (`KismetSystemLibrary.DoesImplementInterface` OtherActor "/Game/BPMobileHorror/Core/Interfaces/BPI_MHInteractInterface.BPI_MHInteractInterface_C")
    (set `self.InteractableInSight` true)
    (message `/Game/BPMobileHorror/Core/Interfaces/BPI_MHInteractInterface.MHReadyToUse` OtherActor true)))

(event `self.InteractCapsule.OnComponentEndOverlap`
  (params (OverlappedComponent :type "PrimitiveComponent Object Reference") (OtherActor :type "Actor Object Reference") (OtherComp :type "PrimitiveComponent Object Reference") (OtherBodyIndex :type Integer))
  (if (`KismetSystemLibrary.DoesImplementInterface` OtherActor "/Game/BPMobileHorror/Core/Interfaces/BPI_MHInteractInterface.BPI_MHInteractInterface_C")
    (set `self.InteractableInSight` false)
    (message `/Game/BPMobileHorror/Core/Interfaces/BPI_MHInteractInterface.MHReadyToUse` OtherActor false)))

(fn `ActionUse`
  ;[1 1 1] Interaction with active objects
  (bind _actortointeract (`self.ActorToInteract`)
    (:`then`
      (bind _success (message `/Game/BPMobileHorror/Core/Interfaces/BPI_MHInteractInterface.MHInteract` _actortointeract))
      (`KismetSystemLibrary.PrintString` (`KismetStringLibrary.Concat_StrStr` (`KismetMathLibrary.SelectString` "Interact " "Not interact " _success) " with " (`KismetSystemLibrary.GetDisplayName` _actortointeract)) true false (`KismetMathLibrary.SelectColor` (struct :`G` 1.0 :`B` 0.082428 :`A` 1.0) (struct :`R` 1.0 :`G` 0.027276 :`A` 1.0) _success) 3.0))
    (:`else`)))

(fn `CheckInteractionActorInSight`
  (locals (L_Actor :type "Actor Object Reference"))
  (bind _returnvalue (`SceneComponent.K2_GetComponentLocation` (`self.PlayerCamera`)))
  (if (`self.InteractableInSight`)
    (bind (_outhit _returnvalue_2) (`KismetSystemLibrary.SphereTraceSingle` :`Start` _returnvalue :`End` (+ _returnvalue (* (`SceneComponent.GetForwardVector` (`self.PlayerCamera`)) (`self.InteractionRadius`))) :`TraceChannel` "TraceTypeQuery1" :`DrawDebugType` "ForOneFrame"))
    (if _returnvalue_2
      (set `local.L_Actor` (`.HitActor` (`GameplayStatics.BreakHitResult` _outhit)))
      (if (`KismetSystemLibrary.DoesImplementInterface` (`local.L_Actor`) "/Game/BPMobileHorror/Core/Interfaces/BPI_MHInteractInterface.BPI_MHInteractInterface_C")
        (`|ExecutionSequence`
          (:`then_0`
            (`self.ActorToInteract`
              (:`then`
                (if (!= (`self.ActorToInteract`) (`local.L_Actor`))
                  (set `self.ActorToInteract` (`local.L_Actor`))))
              (:`else`
                (set `self.ActorToInteract` (`local.L_Actor`)))))
          (:`then_1`
            (message `/Game/BPMobileHorror/Core/Interfaces/BPI_MHInteractInterface.MHReadyToUse` (`self.ActorToInteract`) true))))
      (else
        (`self.ActorToInteract`
          (:`then`
            (set `self.ActorToInteract` null))
          (:`else`))))))

(fn `UpdateInteractionRadius`
  (set `self.InteractionRadius` (* (`CapsuleComponent.CapsuleHalfHeight` (`self.InteractCapsule`)) 2.0)))

(fn `UserConstructionScript`
  (`parent.UserConstructionScript`))