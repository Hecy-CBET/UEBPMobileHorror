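; Base door Blueprint for a mobile horror game, with an interact hook that returns false by default.
; The construction script yaws the DoorRotator by the max open angle when the door is flagged open.
; A box collision toggles the hint scene and its children when a player character base enters or leaves, and hints start hidden on BeginPlay.
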(event `self.ReceiveBeginPlay`
  (`self.UpdateHintsVisibility` false))

(event `self.BoxCollisionForInteract.OnComponentBeginOverlap`
  (params (OverlappedComponent :type "PrimitiveComponent Object Reference") (OtherActor :type "Actor Object Reference") (OtherComp :type "PrimitiveComponent Object Reference") (OtherBodyIndex :type Integer) (bFromSweep :type Boolean) (SweepResult :type "HitResult Structure (by ref)"))
  (cast `/Game/BPMobileHorror/Core/Pawns/BP_MHCharacterBase` OtherActor)
  (`self.UpdateHintsVisibility` true))

(event `self.BoxCollisionForInteract.OnComponentEndOverlap`
  (params (OverlappedComponent :type "PrimitiveComponent Object Reference") (OtherActor :type "Actor Object Reference") (OtherComp :type "PrimitiveComponent Object Reference") (OtherBodyIndex :type Integer))
  (cast `/Game/BPMobileHorror/Core/Pawns/BP_MHCharacterBase` OtherActor)
  (`self.UpdateHintsVisibility` false))

(fn `MHInteract`
  (returns (Success :type Boolean))
  (return false))

(fn `UpdateHintsVisibility`
  (params (InVisible :type Boolean))
  (`SceneComponent.SetVisibility` (`self.HintScene`) InVisible true))

(fn `UserConstructionScript`
  (`SceneComponent.K2_AddRelativeRotation` (`self.DoorRotator`) (`KismetMathLibrary.MakeRotator` 0.0 0.0 (`KismetMathLibrary.SelectFloat` (`self.MaxDoorOpenAngle`) 0.0 (`self.IsDoorOpen`))) false false))