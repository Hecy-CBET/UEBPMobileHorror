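; BP_MHDoorBase is an interactable hinged door for the mobile horror game, showing hint components when ready to interact.
; MHInteract finds the overlapping player and uses a dot product to pick the swing direction from their side.
; SwitchOpen plays or reverses a timeline driving the rotator's yaw, keeping the swing direction when interrupted mid-motion.
; The construction script pre-rotates doors flagged as open.
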(event `self.ReceiveBeginPlay`
  (`self.UpdateHintsVisibility` false))

(event `/Game/BPMobileHorror/Core/Interfaces/BPI_MHInteractInterface.MHReadyToUse`
  (params (InReadyToUse :type Boolean))
  (set `self.IsReadyToInteract` InReadyToUse)
  (`self.UpdateHintsVisibility` (`self.IsReadyToInteract`)))

(event `SwitchOpen`
  (bind _output_get (set `self.IsDoorOpen` (not (`self.IsDoorOpen`))))
  (if _output_get
    (bind (_direction _openprogression) (`Timeline|DoorOpenTimeline` :!label _label)
      (:`Update`
        (set `self.InProgress` true)
        (`self.UpdateDoorRotator` _openprogression))
      (:`Finished`
        (set `self.InProgress` false)))
    (else
      (goto _label :!via `Reverse`))))

(fn `MHInteract`
  (returns (Success :type Boolean))
  (locals (L_DotResult :type Boolean))
  (bind _overlappingactors (`PrimitiveComponent.GetOverlappingActors` (`self.BoxCollision`) "/Game/BPMobileHorror/Core/Pawns/Player/BP_MHPlayerCharacter.BP_MHPlayerCharacter_C"))
  (bind (_relativerotation_roll _relativerotation_pitch _relativerotation_yaw) (`KismetMathLibrary.BreakRotator` (`SceneComponent.RelativeRotation` (`self.DoorRotator`))))
  (bind _output (`|GetArrayItem` _overlappingactors))
  (`|ExecutionSequence`
    (:`then_0`
      (if (`KismetArrayLibrary.Array_IsValidIndex` _overlappingactors)
        (if (`KismetSystemLibrary.IsValid` _output)
          (set `local.L_DotResult` (< (`KismetMathLibrary.Dot_VectorVector` (`self.GetActorForwardVector`) (`KismetMathLibrary.GetForwardVector` (`KismetMathLibrary.FindLookAtRotation` (`self.K2_GetActorLocation`) (`self.K2_GetActorLocation` _output)))) 0.0))
          (if (not (`self.InProgress`))
            (if (not (`self.IsDoorOpen`))
              (set `self.IsFrontOfDoor` (`local.L_DotResult`))
              (else
                (set `self.IsFrontOfDoor` (>= _relativerotation_yaw 0.0))))
            (set `self.PreviousIsFrontOfDoor` (`self.IsFrontOfDoor`))
            (`self.SwitchOpen`)
            (return true)
            (else
              (set `self.IsFrontOfDoor` (`self.PreviousIsFrontOfDoor`))
              (`self.SwitchOpen`)
              (return true))))))
    (:`then_1`
      (return false))))

(fn `UpdateDoorRotator`
  (params (InOpenMult :type "Float (double-precision)"))
  (`SceneComponent.K2_SetRelativeRotation` (`self.DoorRotator`) (`KismetMathLibrary.MakeRotator` 0.0 0.0 (* (`KismetMathLibrary.SelectFloat` (`self.MaxDoorOpenAngle`) (* (`self.MaxDoorOpenAngle`) -1.0) (`self.IsFrontOfDoor`)) (`local.InOpenMult`))) false false))

(fn `UpdateHints`
  (`self.UpdateHintsVisibility` (`self.IsReadyToInteract`)))

(fn `UpdateHintsVisibility`
  (params (InVisible :type Boolean))
  (`SceneComponent.SetVisibility` (`self.HintScene`) (`local.InVisible`) true))

(fn `UserConstructionScript`
  (`SceneComponent.K2_AddRelativeRotation` (`self.DoorRotator`) (`KismetMathLibrary.MakeRotator` 0.0 0.0 (`KismetMathLibrary.SelectFloat` (`self.MaxDoorOpenAngle`) 0.0 (`self.IsDoorOpen`))) false false))